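; BP_HealthPack is a health pickup that restores a fixed amount of life to BP_Player on overlap.
; BodyZone overlap adds to the player's CurrentLifeValue, clamped to MaxLifeValue, while a separate TriggerZone overlap destroys the pack after a short delay.
; Tick spins the skeletal mesh in pitch by RotateSpeed, scaled by a random factor re-rolled each frame.
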(event OnComponentBeginOverlap(TriggerZone)
  (params (OverlappedComponent :type Primitive%20Component%20Object%20Reference) (OtherActor :type Actor%20Object%20Reference) (OtherComp :type Primitive%20Component%20Object%20Reference) (OtherBodyIndex :type Integer) (bFromSweep :type Boolean) (SweepResult :type Hit%20Result%20Structure%20%28by%20ref%29))
  (Utilities|Casting|CastToBP_Player OtherActor)
  (Utilities|FlowControl|Delay 0.1)
  (Actor|DestroyActor))

(event OnComponentBeginOverlap(BodyZone)
  (params (OverlappedComponent :type Primitive%20Component%20Object%20Reference) (OtherActor :type Actor%20Object%20Reference) (OtherComp :type Primitive%20Component%20Object%20Reference) (OtherBodyIndex :type Integer) (bFromSweep :type Boolean) (SweepResult :type Hit%20Result%20Structure%20%28by%20ref%29))
  (bind _asbp_player (Utilities|Casting|CastToBP_Player OtherActor))
  (Variables|/Game/InfiniteMatrix/Blueprints/BP_Player.BP_Player_C|SetCurrentLifeValue _asbp_player (Math|Float|Clamp(Float) (+ (Variables|/Game/InfiniteMatrix/Blueprints/BP_Player.BP_Player_C|GetCurrentLifeValue _asbp_player) 2.0) 0.0 (Variables|/Game/InfiniteMatrix/Blueprints/BP_Player.BP_Player_C|GetMaxLifeValue _asbp_player))))

(event EventBeginPlay)

(event Collision|EventActorBeginOverlap
  (params (OtherActor :type Actor%20Object%20Reference)))

(event EventTick
  (params (DeltaSeconds :type Float%20%28single-precision%29))
  (Transformation|AddLocalRotation (Variables|SkeletalMeshActor|GetSkeletalMeshComponent) (Math|Rotator|MakeRotator 0.0 (* DeltaSeconds (Variables|Default|GetRotateSpeed) (Math|Random|RandomFloatinRange 0.1 5.0)) 0.0) false false))

(fn ConstructionScript)